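; Hover component that pushes a physics-driven parent away from the surface below it, acting as a hover spring.
; Each tick it traces along its negative up vector, with debug drawing, and applies force along the hit normal at its location, fading linearly with distance.
; InitComponent prints the parent component chain and enables physics on ParentComponent, but the node assigning that variable from MeshComponent is disconnected.
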(event Custom|InitComponent
  (params (Mesh_Component :type Static%20Mesh%20Component%20Object%20Reference))
  (for _array_element (Class|SceneComponent|GetParentComponents (stale _output_get))
    (Development|PrintString (Utilities|GetDisplayName _array_element))
    (Physics|SetSimulatePhysics (stale _output_get) true)))

(event EventTick
  (params (DeltaSeconds :type Float%20%28single-precision%29))
  (bind _returnvalue (Transformation|GetWorldLocation))
  (bind (_outhit _returnvalue_2) (Collision|LineTraceByChannel _returnvalue (+ _returnvalue (* (Math|Vector|GetUpVector) (* (Variables|Default|GetTraceLength%20) -1.0)) "0,0.000000,0") "TraceTypeQuery1" true 0 "ForDuration"))
  (if _returnvalue_2
    (Class|PrimitiveComponent|AddForceatLocation (Variables|Default|GetParent_Component) (* (.ImpactNormal (Collision|BreakHitResult _outhit)) (Math|Float|Lerp (Variables|Default|GetHoverForce) 0.0 (/ (Math|Vector|VectorLength (- (.Location (Collision|BreakHitResult _outhit)) (Transformation|GetWorldLocation))) (Variables|Default|GetTraceLength%20)))) (Transformation|GetWorldLocation) "None")))